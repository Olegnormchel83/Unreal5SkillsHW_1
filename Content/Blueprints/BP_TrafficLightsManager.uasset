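; Manager Blueprint that cycles an array of traffic lights like a junction, with even and odd indices showing opposite red and green.
; BeginPlay sets the starting colors, then a Delay loop repeatedly turns all lights yellow before swapping the two groups.
; Helpers pass colors to each light's ChangeColor, picking them by position from the ColorSettings map values.
; An earlier solution that switches all lights in unison remains disconnected.
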(event `self.ReceiveBeginPlay`
  (`self.Recolor`))

(event `Recolor`
  (bind _trafficlights (`self.TrafficLights`))
  ;[1 1 1] Recolor Solution #2. Переключение по логике работы перекрестка
  (if (`KismetArrayLibrary.Array_IsNotEmpty` _trafficlights)
    (for (_array_element _array_index) _trafficlights
      (`self.SetDefaultColors` _array_element _array_index) ; Установка цветов по умолчанию по принципу: четный - красный, нечетный - зеленый
    )
    (`KismetSystemLibrary.Delay` 3.0 :!label _label)
    (`self.ChangeAllTraficLightsColor` _trafficlights) ; Смена цветов по принципу: все стали желытми -> четные стали зелеными -> все стали желтыми -> четные стали красными, как в самом начале, а дальше по новой
    (goto _label)))

(fn `SetDefaultColors`
  (params (TrafficLight :type "/Game/Blueprints/BP_TraffictLight Object Reference") (TrafficLightsArrayIndex :type Integer))
  (if (== (mod TrafficLightsArrayIndex 2) 0)
    (`self.SetRedColor` TrafficLight)
    (else
      (`self.SetGreenColor` TrafficLight))))

(fn `SetGreenColor`
  (params (TrafficLight :type "/Game/Blueprints/BP_TraffictLight Object Reference"))
  (bind _colorsettings_colormap (break `/Game/Blueprints/S_LIghtColor` (`self.ColorSettings`)))
  (bind _values (`BlueprintMapLibrary.Map_Values` _colorsettings_colormap))
  (`/Game/Blueprints/BP_TraffictLight.ChangeColor` TrafficLight (`|GetArrayItem` _values))
  (return))

(fn `SetRedColor`
  (params (TrafficLight :type "/Game/Blueprints/BP_TraffictLight Object Reference"))
  (bind _colorsettings_colormap (break `/Game/Blueprints/S_LIghtColor` (`self.ColorSettings`)))
  (bind _values (`BlueprintMapLibrary.Map_Values` _colorsettings_colormap))
  (`/Game/Blueprints/BP_TraffictLight.ChangeColor` TrafficLight (`|GetArrayItem` _values 2))
  (return))

(fn `SetYellowColor`
  (params (TrafficLight :type "/Game/Blueprints/BP_TraffictLight Object Reference"))
  (bind _colorsettings_colormap (break `/Game/Blueprints/S_LIghtColor` (`self.ColorSettings`)))
  (bind _values (`BlueprintMapLibrary.Map_Values` _colorsettings_colormap))
  (`/Game/Blueprints/BP_TraffictLight.ChangeColor` TrafficLight (`|GetArrayItem` _values 1))
  (return))

(fn `UserConstructionScript`)